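; ItemMap is an inventory item that shows an old map on screen when used and destroys itself once read.
; On use it disables the inventory widget, adds an OldMap widget centred on the main widget's canvas with itself as owner, and switches to UI-only input.
; OnRead re-enables the inventory, removes the map, restores game-and-UI input and destroys the actor.
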(event `self.EventOnUsed`
  (`Widget.SetIsEnabled` (`/Game/InventorySystem/Widgets/MainWidget.InventoryWidget` (`/Game/InventorySystem/Blueprints/BP_Inventory.MainWidget` (`self.Inventory`))) false)
  (bind _returnvalue (`|CreateWidget` "/Game/InventorySystem/Widgets/OldMap.OldMap_C" null self))
  (bind _output_get (set `self.MapWidget` _returnvalue))
  (bind _returnvalue_2 (`CanvasPanel.AddChildToCanvas` (`/Game/InventorySystem/Widgets/MainWidget.Canvas` (`/Game/InventorySystem/Blueprints/BP_Inventory.MainWidget` (`self.Inventory`))) _output_get))
  (`CanvasPanelSlot.SetAnchors` _returnvalue_2 (make `Anchors` (0.5 0.5) (0.5 0.5)))
  (`CanvasPanelSlot.SetAutoSize` _returnvalue_2 true)
  (`CanvasPanelSlot.SetPosition` _returnvalue_2 (-325.0 -240.0))
  (`WidgetBlueprintLibrary.SetInputMode_UIOnlyEx` (`GameplayStatics.GetPlayerController` 0) (`self.MapWidget`)))

(event `OnRead`
  (`Widget.SetIsEnabled` (`/Game/InventorySystem/Widgets/MainWidget.InventoryWidget` (`/Game/InventorySystem/Blueprints/BP_Inventory.MainWidget` (`self.Inventory`))) true)
  (`Widget.RemoveFromParent` (`self.MapWidget`))
  (`WidgetBlueprintLibrary.SetInputMode_GameAndUIEx` (`GameplayStatics.GetPlayerController` 0) null "DoNotLock" false)
  (`self.K2_DestroyActor`))

(fn `UserConstructionScript`
  (`parent.UserConstructionScript`))