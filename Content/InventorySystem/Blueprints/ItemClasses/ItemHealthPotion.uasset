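; ItemHealthPotion is an inventory item that restores a fixed amount of health to the player character when used.
; Its used event reads current and max HP through the inventory's character reference and, if below max, heals and removes one potion at its inventory index.
; The item actor destroys itself in either case, but at full health the inventory is left untouched.
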(event `self.EventOnUsed`
  (bind _mycharacterref (`/Game/InventorySystem/Blueprints/BP_Inventory.MyCharacterRef` (`self.Inventory`)))
  (if (< (`/Game/TopDownBP/Blueprints/MyCharacter.CurrentHP` _mycharacterref) (`/Game/TopDownBP/Blueprints/MyCharacter.MaxHP` _mycharacterref))
    (`/Game/TopDownBP/Blueprints/MyCharacter.IncreaseHealth` _mycharacterref 10)
    (`/Game/InventorySystem/Blueprints/BP_Inventory.RemoveItemAtIndex` (`self.Inventory`) (`self.Index`) 1)
    (`self.K2_DestroyActor`)
    (else
      (`self.K2_DestroyActor`))))

(fn `UserConstructionScript`
  (`parent.UserConstructionScript`))